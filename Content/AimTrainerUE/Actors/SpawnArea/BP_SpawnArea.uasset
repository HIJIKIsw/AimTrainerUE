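; BP_SpawnArea is an aim-trainer actor that periodically spawns BP_Target actors at random points inside a box volume.
; Tick counts down a timer, resets it to one second when it expires, then spawns a target with zero rotation and unit scale.
; The spawn point comes from the SpawnAreaBox world location and unscaled extent, so the box's rotation and scale do not affect the area.
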(event `self.ReceiveTick`
  (params (DeltaSeconds :type "Float (single-precision)"))
  (bind _untilspawntargetseconds (`self.UntilSpawnTargetSeconds`))
  (bind _spawnareabox (`self.SpawnAreaBox`))
  (bind _returnvalue_location (`KismetMathLibrary.BreakTransform` (`SceneComponent.K2_GetComponentToWorld` _spawnareabox)))
  (set `self.UntilSpawnTargetSeconds` (- _untilspawntargetseconds DeltaSeconds))
  (if (<= _untilspawntargetseconds 0.0)
    (set `self.UntilSpawnTargetSeconds` 1.0)
    (`|SpawnActorFromClass` "/Game/AimTrainerUE/Actors/Targets/BP_Target.BP_Target_C" (`KismetMathLibrary.MakeTransform` (`KismetMathLibrary.RandomPointInBoundingBox` _returnvalue_location (`BoxComponent.GetUnscaledBoxExtent` _spawnareabox))) "Undefined" "MultiplyWithRoot" null null)))

(fn `UserConstructionScript`)