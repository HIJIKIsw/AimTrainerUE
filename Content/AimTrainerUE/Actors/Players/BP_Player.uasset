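; BP_Player is the player Blueprint for an aim trainer, handling movement, look and hitscan shooting through Enhanced Input.
; On BeginPlay it adds the input mapping context to the local player.
; Move input follows control rotation, and look input is scaled by LookSensitivity.
; Each fire press runs a long Visibility line trace from the camera, draws it for debugging and applies fixed damage to the hit actor.
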(event `self.ReceiveBeginPlay`
  (bind `_asプレイヤーコントローラー` (cast `PlayerController` (`self.GetController`)))
  (`EnhancedInputSubsystemInterface.AddMappingContext` (pcsubsystem `EnhancedInputLocalPlayerSubsystem` `_asプレイヤーコントローラー`) "/Game/AimTrainerUE/Inputs/IMC_Input.IMC_Input" 0 (struct)))

(event `EnhancedInput|/Game/AimTrainerUE/Inputs/IA_Move`
  (params (ActionValue :type "Vector2D Structure") (ElapsedSeconds :type "Float (double-precision)") (TriggeredSeconds :type "Float (double-precision)") (InputAction :type "InputAction Object Reference" :default "/Game/AimTrainerUE/Inputs/IA_Move.IA_Move"))
  (bind _returnvalue (`self.GetControlRotation`))
  (:`Triggered`
    (`self.AddMovementInput` (`KismetMathLibrary.GetForwardVector` _returnvalue) ActionValue_X)
    (`self.AddMovementInput` (`KismetMathLibrary.GetRightVector` _returnvalue) ActionValue_Y)))

(event `EnhancedInput|/Game/AimTrainerUE/Inputs/IA_Look`
  (params (ActionValue :type "Vector2D Structure") (ElapsedSeconds :type "Float (double-precision)") (TriggeredSeconds :type "Float (double-precision)") (InputAction :type "InputAction Object Reference" :default "/Game/AimTrainerUE/Inputs/IA_Look.IA_Look"))
  (bind _looksensitivity (`self.LookSensitivity`))
  (:`Triggered`
    (`self.AddControllerPitchInput` (* ActionValue_Y _looksensitivity))
    (`self.AddControllerYawInput` (* ActionValue_X _looksensitivity))))

(event `EnhancedInput|/Game/AimTrainerUE/Inputs/IA_Fire`
  (params (ActionValue :type Boolean) (ElapsedSeconds :type "Float (double-precision)") (TriggeredSeconds :type "Float (double-precision)") (InputAction :type "InputAction Object Reference" :default "/Game/AimTrainerUE/Inputs/IA_Fire.IA_Fire"))
  (bind _camera (`self.Camera`))
  (bind _returnvalue (`SceneComponent.K2_GetComponentLocation` _camera))
  (:`Started`
    (bind (_outhit _returnvalue_2) (`KismetSystemLibrary.LineTraceSingle` :`Start` _returnvalue :`End` (+ _returnvalue (* (`SceneComponent.GetForwardVector` _camera) (100000.0 100000.0 100000.0))) :`TraceChannel` "TraceTypeQuery1" :`DrawDebugType` "ForDuration" :`DrawTime` 1.0))
    (if _returnvalue_2
      (`GameplayStatics.ApplyDamage` (`.HitActor` (`GameplayStatics.BreakHitResult` _outhit)) 100.0))))

(fn `UserConstructionScript`)